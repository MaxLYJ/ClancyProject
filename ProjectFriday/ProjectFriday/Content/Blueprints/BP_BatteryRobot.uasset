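; BP_BatteryRobot is a robot that counts installed batteries and flags the day's battery goal as complete.
; Box overlap toggles the Battery component's visibility and gives the first-person character a proximity flag and robot reference.
; SetBatteryNum increments the string-stored count and refreshes the current/max text.
; At max, it prints a win message and sets BP_TimeManager's Day 1 or Day 2 completion flag according to BotAppearDayNum.
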(event `self.ReceiveBeginPlay`
  (`TextRenderComponent.K2_SetText` (`self.BatteryNumber`) (`KismetTextLibrary.Conv_StringToText` (`KismetStringLibrary.Concat_StrStr` (`self.CurrentBatteryNum`) "/" (`self.MaxBatteryNum`))))
  (bind _asbp_first_person_character (cast `/Game/FirstPerson/Blueprints/BP_FirstPersonCharacter` (`GameplayStatics.GetPlayerCharacter` 0)))
  (set `self.As BP First Person Character` _asbp_first_person_character)
  (bind _returnvalue (`GameplayStatics.GetActorOfClass` "/Game/Blueprints/BP_TimeManager.BP_TimeManager_C"))
  (set `self.AsTimeManager` _returnvalue))

(event `self.Box.OnComponentBeginOverlap`
  (params (OverlappedComponent :type "PrimitiveComponent Object Reference") (OtherActor :type "Actor Object Reference") (OtherComp :type "PrimitiveComponent Object Reference") (OtherBodyIndex :type Integer) (bFromSweep :type Boolean) (SweepResult :type "HitResult Structure (by ref)"))
  (bind _asbp_first_person_character (cast `/Game/FirstPerson/Blueprints/BP_FirstPersonCharacter` OtherActor))
  (`SceneComponent.SetVisibility` (`self.Battery`) true false)
  (set `/Game/FirstPerson/Blueprints/BP_FirstPersonCharacter.IsNearBatteryRobot` true _asbp_first_person_character)
  (set `/Game/FirstPerson/Blueprints/BP_FirstPersonCharacter.bp_BatteryRobot` self _asbp_first_person_character))

(event `self.Box.OnComponentEndOverlap`
  (params (OverlappedComponent :type "PrimitiveComponent Object Reference") (OtherActor :type "Actor Object Reference") (OtherComp :type "PrimitiveComponent Object Reference") (OtherBodyIndex :type Integer))
  (bind _asbp_first_person_character (cast `/Game/FirstPerson/Blueprints/BP_FirstPersonCharacter` OtherActor))
  (`SceneComponent.SetVisibility` (`self.Battery`) false false)
  (set `/Game/FirstPerson/Blueprints/BP_FirstPersonCharacter.IsNearBatteryRobot` false _asbp_first_person_character)
  (set `/Game/FirstPerson/Blueprints/BP_FirstPersonCharacter.bp_BatteryRobot` null _asbp_first_person_character))

(fn `SetBatteryNum`
  (bind _result (`/Engine/EditorBlueprintResources/StandardMacros.IncrementInt` (`KismetStringLibrary.Conv_StringToInt` (`self.CurrentBatteryNum`)))
    (:`  `
      (set `self.CurrentBatteryNum` (`KismetStringLibrary.Conv_IntToString` _result))
      (`TextRenderComponent.K2_SetText` (`self.BatteryNumber`) (`KismetTextLibrary.Conv_StringToText` (`KismetStringLibrary.Concat_StrStr` (`self.CurrentBatteryNum`) "/" (`self.MaxBatteryNum`))))
      (if (`KismetStringLibrary.EqualEqual_StrStr` (`self.CurrentBatteryNum`) (`self.MaxBatteryNum`))
        (`KismetSystemLibrary.PrintString` "YouWin")
        (if (== (`self.BotAppearDayNum`) 1)
          (set `/Game/Blueprints/BP_TimeManager.isDay1InstallAllBatteries` true (`self.AsTimeManager`))
          (elif (== (`self.BotAppearDayNum`) 2)
            (set `/Game/Blueprints/BP_TimeManager.isDay2InstallAllBatteries` true (`self.AsTimeManager`))))))))

(fn `UserConstructionScript`)