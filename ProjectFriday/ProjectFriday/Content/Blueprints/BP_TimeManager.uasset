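; Time manager actor that runs the day countdown and opens the Gameover level when anomalies fill every selection slot.
; A looping one-second timer decrements the countdown and counts existing entries in the SelectionMaster's StrucSelection array to test for that loss.
; When the countdown expires, it resets, advances the day and calls TimeUp with the new day.
; On that expiry tick the anomaly count is zeroed before the loss check.
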(event `self.ReceiveBeginPlay`
  (`|ExecutionSequence`
    (:`then_0`
      (bind _returnvalue (`GameplayStatics.GetActorOfClass` "/Game/FirstPerson/Blueprints/BP_SelectionMaster.BP_SelectionMaster_C"))
      (set `self.selectionMaster` _returnvalue))
    (:`then_1`
      (set `self.CurrentDay` 1)
      (set `self.CurrentCountdown` 50)
      (`KismetSystemLibrary.K2_SetTimerDelegate` (delegate `Countdown`) 1.0 true))))

(event `Countdown`
  (bind _returnvalue (>= (`self.CurrentAnomly`) (`KismetArrayLibrary.Array_Length` (`/Game/FirstPerson/Blueprints/BP_SelectionMaster.StrucSelection` (`self.selectionMaster`)))))
  (for _array_element (`/Game/FirstPerson/Blueprints/BP_SelectionMaster.StrucSelection` (`self.selectionMaster`))
    (if (`.IfExist_6_9F9B4E5042AD99F11DB615ADE61DAFE3` (break `/Game/Widgets/Struc_SelectOption` _array_element))
      (`/Engine/EditorBlueprintResources/StandardMacros.IncrementInt` (`self.CurrentAnomly`))))
  (bind _result (`/Engine/EditorBlueprintResources/StandardMacros.DecrementInt` (`self.CurrentCountdown`))
    (:`  `
      (bind _output_get (set `self.CurrentCountdown` _result))
      (bind _output_get_2 (set `self.CountdownEnd` (< _output_get 1)))
      (if _output_get_2
        (set `self.CurrentAnomly` 0)
        (set `self.CurrentCountdown` 50)
        (if _returnvalue
          (`GameplayStatics.OpenLevel` "Gameover")
          (else
            (bind _result_2 (`/Engine/EditorBlueprintResources/StandardMacros.IncrementInt` (`self.CurrentDay`))
              (:`  `
                (set `self.CurrentDay` _result_2)
                (`self.TimeUp` (`self.CurrentDay`))))))
        (elif _returnvalue
          (`GameplayStatics.OpenLevel` "Gameover")
          (else
            (set `self.CurrentAnomly` 0)))))))

(fn `UserConstructionScript`)